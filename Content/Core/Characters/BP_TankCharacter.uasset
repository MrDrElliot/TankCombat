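; Player character Blueprint with tank-style controls, where movement input turns the character and drives it along its facing direction.
; On BeginPlay, a locally controlled instance adds the default Enhanced Input mapping context to player controller 0.
; The move action's X axis becomes clamped controller yaw and its Y axis scales movement along the actor's forward vector.
; The zoom action passes its value to UpdateZoom, which is defined outside these graphs.
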(event `self.ReceiveBeginPlay`
  (`self.SetupLocalInputs`))

(event `EnhancedInput|/Game/Core/Input/IA_Move`
  (params (ActionValue :type "Vector2D Structure") (ElapsedSeconds :type "Float (double-precision)") (TriggeredSeconds :type "Float (double-precision)") (InputAction :type "InputAction Object Reference" :default "/Game/Core/Input/IA_Move.IA_Move"))
  (:`Triggered`
    (`self.AddControllerYawInput` (`KismetMathLibrary.FClamp` ActionValue_X -0.3 0.3))
    (`self.AddMovementInput` (`self.GetActorForwardVector`) ActionValue_Y)))

(event `EnhancedInput|/Game/Core/Input/IA_Zoom`
  (params (ActionValue :type "Float (double-precision)") (ElapsedSeconds :type "Float (double-precision)") (TriggeredSeconds :type "Float (double-precision)") (InputAction :type "InputAction Object Reference" :default "/Game/Core/Input/IA_Zoom.IA_Zoom"))
  (:`Triggered`
    (`self.UpdateZoom` ActionValue)))

(fn `SetupLocalInputs`
  (if (`self.IsLocallyControlled`)
    (`EnhancedInputSubsystemInterface.AddMappingContext` (pcsubsystem `EnhancedInputLocalPlayerSubsystem` (`GameplayStatics.GetPlayerController` 0)) "/Game/Core/Input/IMC_Default.IMC_Default" 0 (struct))))

(fn `UserConstructionScript`)